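; Player controller Blueprint that creates and manages the player's HUD and inventory widgets.
; On BeginPlay it casts the player character to MainCharacter_BP, then creates both widgets, showing the HUD only when the level is not MainMenu.
; The Inventory input action uses a FlipFlop to toggle the inventory widget on and off the viewport.
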(event `self.ReceiveBeginPlay`
  (`self.CreateWidgets`))

(event `InputAction|Inventory`
  (params (Key :type "Key Structure"))
  (:`Pressed`
    (`/Engine/EditorBlueprintResources/StandardMacros.FlipFlop`
      (:`A`
        (`UserWidget.AddToViewport` (`self.Inventory`) 0))
      (:`B`
        (`Widget.RemoveFromParent` (`self.Inventory`))))))

(fn `CreateWidgets`
  (`|ExecutionSequence`
    (:`then_0`
      (cast `/Game/Characters/Player/MainCharacter_BP` (`GameplayStatics.GetPlayerCharacter` 0))
      (set `self.PlayerRef` (`self.PlayerRef`)))
    (:`then_1`
      (bind _returnvalue (`|CreateWidget` "/Game/UI/PlayerHUD.PlayerHUD_C"))
      (set `self.PlayerHUD` _returnvalue)
      (bind _returnvalue_2 (`GameplayStatics.GetCurrentLevelName` true))
      (if (`KismetStringLibrary.NotEqual_StrStr` _returnvalue_2 "MainMenu")
        (`UserWidget.AddToViewport` (`self.PlayerHUD`) 0)))
    (:`then_2`
      (bind _returnvalue_3 (`|CreateWidget` "/Game/UI/Inventory/Inventory.Inventory_C"))
      (set `self.Inventory` _returnvalue_3))))

(fn `UserConstructionScript`)